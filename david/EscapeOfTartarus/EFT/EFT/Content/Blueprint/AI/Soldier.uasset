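; Soldier is a 2D Paper2D enemy that patrols between two points and damages Joey on contact.
; The Construction Script feeds points A and B to InterpToMovement, and each reversal flip-flops the sprite's yaw.
; Tick picks one of two flipbooks by velocity, while a box overlap applies damage to Joey.
; Health functions and Direction are empty with disconnected logic, and an uncalled Flipbook function holds Joey's directional animation.
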(event OnInterptoReverse(InterpToMovement)
  (params (ImpactResult :type Hit%20Result%20Structure%20%28by%20ref%29) (Time :type Float%20%28single-precision%29))
  (bind _sprite (Variables|Default|GetSprite))
  (Utilities|FlowControl|FlipFlop
    (:A
      (Transformation|SetWorldRotation _sprite "0,180.000000, 0" false false))
    (:B
      (Transformation|SetWorldRotation _sprite "0, 0, 0" false false))))

(event OnComponentBeginOverlap(Box)
  (params (OverlappedComponent :type Primitive%20Component%20Object%20Reference) (OtherActor :type Actor%20Object%20Reference) (OtherComp :type Primitive%20Component%20Object%20Reference) (OtherBodyIndex :type Integer) (bFromSweep :type Boolean) (SweepResult :type Hit%20Result%20Structure%20%28by%20ref%29))
  ;[1 1 1] Attack
  (bind _asjoey (Utilities|Casting|CastToJoey OtherActor))
  (Game|Damage|ApplyDamage _asjoey 5.0 0 0 "/Script/Engine.DamageType"))

(event Custom|Direction
  ;[1 1 1] Enemy Movement
)

(event Custom|Animation
  ;[1 1 1] Animation
  (Sprite|SetFlipbook (Variables|Default|GetSprite) (select (> (Math|Vector|VectorLength (Transformation|GetVelocity)) 0.0) "/Game/Spritesheet/AI_Flipbook/left/soldierleft.soldierleft" "/Game/Spritesheet/AI_Flipbook/right/Soldierright.Soldierright")))

(event EventTick
  (params (DeltaSeconds :type Float%20%28single-precision%29))
  (CallFunction|Direction)
  (CallFunction|Animation))

(fn ConstructionScript
  (Variables|/Script/Engine.InterpToMovementComponent|SetControlPoints (Variables|Default|GetInterpToMovement) (Utilities|Array|MakeArray (Utilities|Struct|MakeInterpControlPoint (Variables|Default|Geta) true) (Utilities|Struct|MakeInterpControlPoint (Variables|Default|Getb) true))))

(fn Flipbook
  ;[1 1 1] Joey's Movement
  (if (or (!= (Input|AxisValues|Getleftandright) 0.0) (!= (Input|AxisValues|Getupanddown) 0.0))
    (Variables|Default|SetJoey_Movements (select (> (Input|AxisValues|Getupanddown) 0.0) "NewEnumerator0" (select (< (Input|AxisValues|Getupanddown) 0.0) "NewEnumerator1" (select (> (Input|AxisValues|Getleftandright) 0.0) "NewEnumerator3" "NewEnumerator2")))))
  (Sprite|SetFlipbook (Variables|Default|GetSprite) (select (> (Math|Vector|VectorLength (Transformation|GetVelocity)) 0.0) (Utilities|Select :Index (Variables|Default|GetJoey_Movements) :NewEnumerator0 "/Game/Spritesheet/MainCharacter_Flipbook/up/up.up" :NewEnumerator1 "/Game/Spritesheet/MainCharacter_Flipbook/down/Down.Down" :NewEnumerator2 "/Game/Spritesheet/MainCharacter_Flipbook/left/left.left" :NewEnumerator3 "/Game/Spritesheet/MainCharacter_Flipbook/right/right.right" :NewEnumerator4 0) (Utilities|Select :Index (Variables|Default|GetJoey_Movements) :NewEnumerator0 "/Game/Spritesheet/MainCharacter_Flipbook/up/idleup.idleup" :NewEnumerator1 "/Game/Spritesheet/MainCharacter_Flipbook/down/idledown.idledown" :NewEnumerator2 "/Game/Spritesheet/MainCharacter_Flipbook/left/idleleft.idleleft" :NewEnumerator3 "/Game/Spritesheet/MainCharacter_Flipbook/right/idleright.idleright" :NewEnumerator4 0))))

(fn EnemyHealth
  (params (Damage :type Integer)))

(fn SoldierHealth
  (params (damage :type Integer)))