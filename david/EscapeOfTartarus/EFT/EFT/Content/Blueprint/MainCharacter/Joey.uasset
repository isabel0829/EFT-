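; Joey is the player's 2D flipbook character, moved along the X and Z axes and shown with a health bar widget.
; Each tick, input and velocity pick a directional walk or idle flipbook; the Attack state has no flipbook assigned there.
; Capsule hits on a Soldier call its health function with -25, regardless of attacking.
; Damage and V/C keys adjust CurrHealth unclamped; other health and animation helpers are unfinished and uncalled here.
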(event OnComponentHit(CapsuleComponent)
  (params (HitComponent :type Primitive%20Component%20Object%20Reference) (OtherActor :type Actor%20Object%20Reference) (OtherComp :type Primitive%20Component%20Object%20Reference) (NormalImpulse :type Vector :default "0, 0, 0") (Hit :type Hit%20Result%20Structure%20%28by%20ref%29))
  ;[1 1 1] Kill Enemy
  (bind _assoldier (Utilities|Casting|CastToSoldier OtherActor))
  (Default|SoldierHealth _assoldier -25))

(event Game|Damage|EventAnyDamage
  (params (Damage :type Float%20%28single-precision%29) (DamageType :type Damage%20Type%20Object%20Reference) (InstigatedBy :type Controller%20Object%20Reference) (DamageCauser :type Actor%20Object%20Reference))
  ;[1 1 1] health
  (Variables|Default|SetCurrHealth (- (Variables|Default|GetCurrHealth) Damage)))

(event EventBeginPlay
  ;[1 1 1] health
  (bind _returnvalue (UserInterface|CreateWidget "/Game/Blueprint/MainCharacter/healthbar.healthbar_C"))
  (bind _output_get (Variables|Default|Sethealthbar _returnvalue))
  (UserInterface|Viewport|AddtoViewport _output_get 0))

(event EventTick
  (params (DeltaSeconds :type Float%20%28single-precision%29))
  ;[1 1 1] Input Movements
  (CallFunction|Flipbook))

(event Input|ActionEvents|InputActionattack
  (params (Key :type Key%20Structure))
  (:Pressed
    (Variables|Default|SetJoey_Movements "NewEnumerator4")))

(event Input|AxisEvents|InputAxisupanddown
  (params (AxisValue :type Float%20%28single-precision%29))
  ;[1 1 1] Input Movements
  (Pawn|Input|AddMovementInput "0, 0,1.000000" AxisValue false))

(event Input|AxisEvents|InputAxisleftandright
  (params (AxisValue :type Float%20%28single-precision%29))
  ;[1 1 1] Input Movements
  (Pawn|Input|AddMovementInput "1.000000, 0, 0" AxisValue false))

(event Input|KeyboardEvents|V
  (params (Key :type Key%20Structure))
  ;[1 1 1] health
  (:Pressed
    (Variables|Default|SetCurrHealth (- (Variables|Default|GetCurrHealth) 5.0))))

(event Input|KeyboardEvents|C
  (params (Key :type Key%20Structure))
  ;[1 1 1] health
  (:Pressed
    (Variables|Default|SetCurrHealth (+ (Variables|Default|GetCurrHealth) 5.0))))

(fn ConstructionScript)

(fn Flipbook
  ;[1 1 1] Joey's Movement
  (if (or (!= (Input|AxisValues|Getleftandright) 0.0) (!= (Input|AxisValues|Getupanddown) 0.0))
    (Variables|Default|SetJoey_Movements (select (> (Input|AxisValues|Getupanddown) 0.0) "NewEnumerator0" (select (< (Input|AxisValues|Getupanddown) 0.0) "NewEnumerator1" (select (> (Input|AxisValues|Getleftandright) 0.0) "NewEnumerator3" "NewEnumerator2")))))
  (Sprite|SetFlipbook (Variables|Default|GetSprite) (select (> (Math|Vector|VectorLength (Transformation|GetVelocity)) 0.0) (Utilities|Select :Index (Variables|Default|GetJoey_Movements) :NewEnumerator0 "/Game/Spritesheet/MainCharacter_Flipbook/up/up.up" :NewEnumerator1 "/Game/Spritesheet/MainCharacter_Flipbook/down/Down.Down" :NewEnumerator2 "/Game/Spritesheet/MainCharacter_Flipbook/left/left.left" :NewEnumerator3 "/Game/Spritesheet/MainCharacter_Flipbook/right/right.right" :NewEnumerator4 0) (Utilities|Select :Index (Variables|Default|GetJoey_Movements) :NewEnumerator0 "/Game/Spritesheet/MainCharacter_Flipbook/up/idleup.idleup" :NewEnumerator1 "/Game/Spritesheet/MainCharacter_Flipbook/down/idledown.idledown" :NewEnumerator2 "/Game/Spritesheet/MainCharacter_Flipbook/left/idleleft.idleleft" :NewEnumerator3 "/Game/Spritesheet/MainCharacter_Flipbook/right/idleright.idleright" :NewEnumerator4 0))))

(fn Changehealth
  (params (amount :type Integer))
  ;[1 1 1] Health Action
)

(fn TakeDamage
  (params (value :type Float%20%28single-precision%29))
  (Variables|Default|SetFullhealth (Math|Float|Clamp(Float) (- (Variables|Default|GetFullhealth) value))))

(fn Animationstatemachine
  (params (ismoving :type Boolean) (isattacking :type Boolean))
  (LocalVariables|Setismovinglocal ismoving)
  (LocalVariables|Setisattackinglocal isattacking)
  (if (LocalVariables|Getisattackinglocal)
    (LocalVariables|SetAnimationstate "NewEnumerator4")
    (elif (LocalVariables|Getismovinglocal)
      (LocalVariables|SetAnimationstate "NewEnumerator0"))))