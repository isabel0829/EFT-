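; BombBP is a pickup item that changes Joey's health and goes into the inventory on overlap.
; It sets its sprite at BeginPlay on a component named Coin, whose overlap applies the health change before attempting to add one CoinStructure item.
; Only a successful add destroys the actor, then a TriggerBox cast gates a sound played at the world origin.
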(event OnComponentBeginOverlap(coin)
  (params (OverlappedComponent :type Primitive%20Component%20Object%20Reference) (OtherActor :type Actor%20Object%20Reference) (OtherComp :type Primitive%20Component%20Object%20Reference) (OtherBodyIndex :type Integer) (bFromSweep :type Boolean) (SweepResult :type Hit%20Result%20Structure%20%28by%20ref%29))
  (bind _asjoey (Utilities|Casting|CastToJoey OtherActor))
  (Default|Changehealth _asjoey (Variables|Default|Gethealthamount))
  (bind _sucess (Default|Addtoinventory (Actor|GetComponentbyClass OtherActor "/Game/Blueprint/Interactive_Object/Chest/Inventory.Inventory_C") (Utilities|Struct|MakeSlotStructure (Variables|Default|GetCoinStructure) 1)))
  (if _sucess
    (Actor|DestroyActor)
    (Utilities|Casting|CastToTriggerBoxClass "/Script/Engine.TriggerBox")
    (Audio|PlaySoundatLocation 0 "0, 0, 0" "0, 0, 0" 1.0 1.0 0.0 0 0 0)))

(event EventBeginPlay
  (Rendering|Components|Sprite|SetSprite (Variables|Default|Getcoin) (Variables|Default|Getmysprite)))

(fn ConstructionScript)