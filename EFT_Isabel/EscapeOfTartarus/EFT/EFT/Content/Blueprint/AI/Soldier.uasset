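; Soldier is a 2D flipbook enemy that patrols between points A and B and changes Joey's health on contact.
; InterpToMovement drives the patrol from construction-script control points, flipping the sprite on each reverse, while Tick picks its flipbook from velocity.
; Duplicate EnemyHealth and SoldierHealth functions add signed damage and destroy it at zero.
; The Direction event is empty, input-based movement is disconnected, and the Joey-style Flipbook function is never called here.
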(event OnComponentHit(CapsuleComponent)
  (params (HitComponent :type Primitive%20Component%20Object%20Reference) (OtherActor :type Actor%20Object%20Reference) (OtherComp :type Primitive%20Component%20Object%20Reference) (NormalImpulse :type Vector :default "0, 0, 0") (Hit :type Hit%20Result%20Structure%20%28by%20ref%29))
  ;[1 1 1] Attack
  (Variables|Default|SetMovingright (not (Variables|Default|GetMovingright)))
  (bind _asjoey (Utilities|Casting|CastToJoey OtherActor))
  (Default|Changehealth _asjoey (Variables|Default|GetHealthAM)))

(event OnInterptoReverse(InterpToMovement)
  (params (ImpactResult :type Hit%20Result%20Structure%20%28by%20ref%29) (Time :type Float%20%28single-precision%29))
  (bind _sprite (Variables|Default|GetSprite))
  ;[1 1 1] Move Direction
  (Utilities|FlowControl|FlipFlop
    (:A
      (Transformation|SetWorldRotation _sprite "0,180.000000, 0" false false))
    (:B
      (Transformation|SetWorldRotation _sprite "0, 0, 0" false false))))

(event Custom|Direction
  ;[1 1 1] Enemy Movement
)

(event Custom|Animation
  ;[1 1 1] Animation
  (Sprite|SetFlipbook (Variables|Default|GetSprite) (select (> (Math|Vector|VectorLength (Transformation|GetVelocity)) 0.0) "/Game/Spritesheet/AI_Flipbook/left/soldierleft.soldierleft" "/Game/Spritesheet/AI_Flipbook/right/Soldierright.Soldierright")))

(event EventBeginPlay
  ;[1 1 1] Health
  (Variables|Default|SetCurAIHealth (Variables|Default|GetMaxAIhealth)))

(event EventTick
  (params (DeltaSeconds :type Float%20%28single-precision%29))
  (CallFunction|Direction)
  (CallFunction|Animation))

(fn ConstructionScript
  (Variables|/Script/Engine.InterpToMovementComponent|SetControlPoints (Variables|Default|GetInterpToMovement) (Utilities|Array|MakeArray (Utilities|Struct|MakeInterpControlPoint (Variables|Default|Geta) true) (Utilities|Struct|MakeInterpControlPoint (Variables|Default|Getb) true))))

(fn Flipbook
  ;[1 1 1] Joey's Movement
  (if (or (!= (Input|AxisValues|Getleftandright) 0.0) (!= (Input|AxisValues|Getupanddown) 0.0))
    (Variables|Default|SetJoey_Movements (select (> (Input|AxisValues|Getupanddown) 0.0) "NewEnumerator0" (select (< (Input|AxisValues|Getupanddown) 0.0) "NewEnumerator1" (select (> (Input|AxisValues|Getleftandright) 0.0) "NewEnumerator3" "NewEnumerator2")))))
  (Sprite|SetFlipbook (Variables|Default|GetSprite) (select (> (Math|Vector|VectorLength (Transformation|GetVelocity)) 0.0) (Utilities|Select :Index (Variables|Default|GetJoey_Movements) :NewEnumerator0 "/Game/Spritesheet/MainCharacter_Flipbook/up/up.up" :NewEnumerator1 "/Game/Spritesheet/MainCharacter_Flipbook/down/Down.Down" :NewEnumerator2 "/Game/Spritesheet/MainCharacter_Flipbook/left/left.left" :NewEnumerator3 "/Game/Spritesheet/MainCharacter_Flipbook/right/right.right") (Utilities|Select :Index (Variables|Default|GetJoey_Movements) :NewEnumerator0 "/Game/Spritesheet/MainCharacter_Flipbook/up/idleup.idleup" :NewEnumerator1 "/Game/Spritesheet/MainCharacter_Flipbook/down/idledown.idledown" :NewEnumerator2 "/Game/Spritesheet/MainCharacter_Flipbook/left/idleleft.idleleft" :NewEnumerator3 "/Game/Spritesheet/MainCharacter_Flipbook/right/idleright.idleright"))))

(fn EnemyHealth
  (params (Damage :type Integer))
  (bind _output_get (Variables|Default|SetCurAIHealth (+ (Variables|Default|GetCurAIHealth) Damage 0)))
  (Development|PrintString (Utilities|String|ToString(Integer) _output_get))
  (if (<= (Variables|Default|GetCurAIHealth) 0)
    (Actor|DestroyActor)))

(fn SoldierHealth
  (params (damage :type Integer))
  (bind _output_get (Variables|Default|SetCurAIHealth (+ (Variables|Default|GetCurAIHealth) damage 0)))
  (Development|PrintString (Utilities|String|ToString(Integer) _output_get))
  (if (<= (Variables|Default|GetCurAIHealth) 0)
    (Actor|DestroyActor)))