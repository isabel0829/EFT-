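; Joey is the Paper2D player character, moving on the X/Z plane with four-direction walk and idle flipbooks updated every tick.
; Capsule hits call SoldierHealth(-10) on Soldiers.
; Health is restored from NewGameInstance and written back by Changehealth (adding Amount twice); at zero, Joey is destroyed and TryAgain appears.
; Input also drives interface-based pickup of overlapping actors, a flip-flop inventory HUD, and saving (S) or loading (1) player location.
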(event OnComponentHit(CapsuleComponent)
  (params (HitComponent :type Primitive%20Component%20Object%20Reference) (OtherActor :type Actor%20Object%20Reference) (OtherComp :type Primitive%20Component%20Object%20Reference) (NormalImpulse :type Vector :default "0, 0, 0") (Hit :type Hit%20Result%20Structure%20%28by%20ref%29))
  ;[1 1 1] Kill Enemy
  (bind _assoldier (Utilities|Casting|CastToSoldier OtherActor))
  (Default|SoldierHealth _assoldier -10))

(event EventBeginPlay
  ;[1 1 1] Health
  (Utilities|FlowControl|Sequence
    (:then_0
      (CallFunction|Createhealthbar))
    (:then_1
      (Variables|Default|Setcurhealth (Variables|Default|Getmaxhealth)))
    (:then_2
      (bind _asnew_game_instance (Utilities|Casting|CastToNewGameInstance (Game|GetGameInstance)))
      (Variables|Default|Setcurhealth (Variables|/Game/Blueprint/SaveandLoad/NewGameInstance.NewGameInstance_C|Gethealthbar _asnew_game_instance)))))

(event EventTick
  (params (DeltaSeconds :type Float%20%28single-precision%29))
  ;[1 1 1] Input Movements
  (CallFunction|Flipbook))

(event Input|ActionEvents|InputActionPickUp
  (params (Key :type Key%20Structure))
  ;[1 1 1] Pick Up Item
  (:Pressed
    (bind _array_element (Utilities|Array|ForEachLoopwithBreak (Collision|GetOverlappingActors 0 :!class /Script/Engine.Actor) :!label _label)
      (:LoopBody
        (if (Utilities|DoesObjectImplementInterface _array_element "/Game/Blueprint/Interactive_Object/Chest/InteractInterface.InteractInterface_C")
          (Class|InteractInterface|Interact(Message) _array_element self)
          (goto _label Break))))))

(event Input|ActionEvents|InputActionInventory
  (params (Key :type Key%20Structure))
  ;[1 1 1] Inventory
  (:Pressed
    (Utilities|FlowControl|FlipFlop
      (:A
        (bind _returnvalue (UserInterface|CreateWidget "/Game/Blueprint/Interactive_Object/Chest/InventoryUI/HUD.HUD_C"))
        (bind _output_get (Variables|Default|SetHudWidget _returnvalue))
        (Default|TogleInventory (Variables|Default|GetInventory))
        (UserInterface|Viewport|AddtoViewport _output_get 0))
      (:B
        (Widget|RemovefromParent (Variables|Default|GetHudWidget))))))

(event Input|AxisEvents|InputAxisupanddown
  (params (AxisValue :type Float%20%28single-precision%29))
  ;[1 1 1] Input Movements
  (Pawn|Input|AddMovementInput "0, 0,1.000000" AxisValue false))

(event Input|AxisEvents|InputAxisleftandright
  (params (AxisValue :type Float%20%28single-precision%29))
  ;[1 1 1] Input Movements
  (Pawn|Input|AddMovementInput "1.000000, 0, 0" AxisValue false))

(event Input|KeyboardEvents|S
  (params (Key :type Key%20Structure))
  ;[1 1 1] Save Player Location
  (:Pressed
    (bind _returnvalue (SaveGame|CreateSaveGameObject "/Game/Blueprint/SaveandLoad/Save_Game.Save_Game_C"))
    (bind _output_get (Variables|Default|SetSave_ref _returnvalue))
    (bind _output_get_2 (Variables|Default|SetPlaye_Loc (Transformation|GetActorLocation)))
    (Variables|/Game/Blueprint/SaveandLoad/Save_Game.Save_Game_C|SetPlayerLocation_Save _output_get _output_get_2)
    (SaveGame|SaveGametoSlot _returnvalue "test")
    (Development|PrintString "Gane Save")))

(event Input|KeyboardEvents|1
  (params (Key :type Key%20Structure))
  ;[1 1 1] Save Player Location
  (:Pressed
    (bind _returnvalue (SaveGame|DoesSaveGameExist "test"))
    (if _returnvalue
      (bind _returnvalue_2 (SaveGame|LoadGamefromSlot "test"))
      (bind _assave_game (Utilities|Casting|CastToSave_Game _returnvalue_2))
      (bind _output_get (Variables|Default|SetPlaye_Loc (Variables|/Game/Blueprint/SaveandLoad/Save_Game.Save_Game_C|GetPlayerLocation_Save _assave_game)))
      (Transformation|SetActorLocation _output_get false false)
      (else
        (Development|PrintString "No Date Exist")))))

(fn ConstructionScript)

(fn Flipbook
  ;[1 1 1] Joey's Movement
  (if (or (!= (Input|AxisValues|Getleftandright) 0.0) (!= (Input|AxisValues|Getupanddown) 0.0))
    (Variables|Default|SetJoey_Movements (select (> (Input|AxisValues|Getupanddown) 0.0) "NewEnumerator0" (select (< (Input|AxisValues|Getupanddown) 0.0) "NewEnumerator1" (select (> (Input|AxisValues|Getleftandright) 0.0) "NewEnumerator3" "NewEnumerator2")))))
  (Sprite|SetFlipbook (Variables|Default|GetSprite) (select (> (Math|Vector|VectorLength (Transformation|GetVelocity)) 0.0) (Utilities|Select :Index (Variables|Default|GetJoey_Movements) :NewEnumerator0 "/Game/Spritesheet/MainCharacter_Flipbook/up/up.up" :NewEnumerator1 "/Game/Spritesheet/MainCharacter_Flipbook/down/Down.Down" :NewEnumerator2 "/Game/Spritesheet/MainCharacter_Flipbook/left/left.left" :NewEnumerator3 "/Game/Spritesheet/MainCharacter_Flipbook/right/right.right") (Utilities|Select :Index (Variables|Default|GetJoey_Movements) :NewEnumerator0 "/Game/Spritesheet/MainCharacter_Flipbook/up/idleup.idleup" :NewEnumerator1 "/Game/Spritesheet/MainCharacter_Flipbook/down/idledown.idledown" :NewEnumerator2 "/Game/Spritesheet/MainCharacter_Flipbook/left/idleleft.idleleft" :NewEnumerator3 "/Game/Spritesheet/MainCharacter_Flipbook/right/idleright.idleright"))))

(fn Changehealth
  (params (amount :type Float%20%28single-precision%29))
  ;[1 1 1] Health Action
  (Utilities|FlowControl|Sequence
    (:then_0
      (bind _output_get (Variables|Default|Setcurhealth (+ (Variables|Default|Getcurhealth) amount)))
      (bind _asnew_game_instance (Utilities|Casting|CastToNewGameInstance (Game|GetGameInstance)))
      (Variables|/Game/Blueprint/SaveandLoad/NewGameInstance.NewGameInstance_C|Sethealthbar _asnew_game_instance (+ (Variables|Default|Getcurhealth) amount))
      (if (<= _output_get 0.0)
        (Actor|DestroyActor)
        (bind _returnvalue (UserInterface|CreateWidget "/Game/Blueprint/MainMenu/TryAgain.TryAgain_C"))
        (UserInterface|Viewport|AddtoViewport _returnvalue 0)))))

(fn Createhealthbar
  (bind _returnvalue (UserInterface|CreateWidget "/Game/Blueprint/HealthBar/HealthBar.HealthBar_C"))
  (bind _output_get (Variables|Default|SetHealthBarReference _returnvalue))
  (UserInterface|Viewport|AddtoViewport _output_get 0))