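; A prison barrier actor that opens by destroying itself when the player character Joey brings the matching key.
; On overlap with its Box, it searches Joey's OwnedKeys for an entry equal to RequiredKeytype and removes it.
; It then copies the remaining keys to PlayerKeys on the TestGameInstance before destroying the actor.
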(event OnComponentBeginOverlap(Box)
  (params (OverlappedComponent :type Primitive%20Component%20Object%20Reference) (OtherActor :type Actor%20Object%20Reference) (OtherComp :type Primitive%20Component%20Object%20Reference) (OtherBodyIndex :type Integer) (bFromSweep :type Boolean) (SweepResult :type Hit%20Result%20Structure%20%28by%20ref%29))
  ;[1 1 1] Open Prison
  (bind _asjoey (Utilities|Casting|CastToJoey OtherActor))
  (for (_array_element _array_index) (Variables|/Game/Blueprint/MainCharacter/Joey.Joey_C|Getowned_keys _asjoey)
    (if (Utilities|Enum|Equal(Enum) _array_element (Variables|Default|Getrequired_keytype))
      (Utilities|Array|RemoveIndex (Variables|/Game/Blueprint/MainCharacter/Joey.Joey_C|Getowned_keys _asjoey) _array_index)
      (bind _astest_game_instance (Utilities|Casting|CastToTestGameInstance (Game|GetGameInstance)))
      (Variables|/Game/TestGameInstance.TestGameInstance_C|Setplayer_Keys _astest_game_instance (Variables|/Game/Blueprint/MainCharacter/Joey.Joey_C|Getowned_keys _asjoey))
      (Actor|DestroyActor))))

(fn ConstructionScript)