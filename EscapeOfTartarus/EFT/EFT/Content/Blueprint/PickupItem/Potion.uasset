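; Health potion pickup actor that changes the player character Joey's health on contact.
; When Joey overlaps its box trigger, it applies its configurable health amount and destroys itself.
; Its sprite comes from a variable, set both in the construction script and again at BeginPlay.
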(event OnComponentBeginOverlap(Box)
  (params (OverlappedComponent :type Primitive%20Component%20Object%20Reference) (OtherActor :type Actor%20Object%20Reference) (OtherComp :type Primitive%20Component%20Object%20Reference) (OtherBodyIndex :type Integer) (bFromSweep :type Boolean) (SweepResult :type Hit%20Result%20Structure%20%28by%20ref%29))
  (bind _asjoey (Utilities|Casting|CastToJoey OtherActor))
  (Default|ChangeHealth _asjoey (Variables|Default|GetHealthamount))
  (Actor|DestroyActor))

(event EventBeginPlay
  (Rendering|Components|Sprite|SetSprite (Variables|Default|Getpotion) (Variables|Default|Getsprite)))

(fn ConstructionScript
  (Rendering|Components|Sprite|SetSprite (Variables|Default|Getpotion) (Variables|Default|Getsprite)))