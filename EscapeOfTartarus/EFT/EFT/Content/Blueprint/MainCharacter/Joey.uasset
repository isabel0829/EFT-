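; Joey is the Paper2D main character, moved by two input axes along world X (left/right) and Z (up/down).
; Each tick, the Flipbook function sets a four-way facing state from the axis values, with vertical input taking priority over horizontal.
; It then picks the moving or idle flipbook for that facing based on whether velocity is non-zero, so the last direction persists when input stops.
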(event EventTick
  (params (DeltaSeconds :type Float%20%28single-precision%29))
  (CallFunction|Flipbook))

(event Input|AxisEvents|InputAxisupanddown
  (params (AxisValue :type Float%20%28single-precision%29))
  (Pawn|Input|AddMovementInput "0, 0,1.000000" AxisValue false))

(event Input|AxisEvents|InputAxisleftandright
  (params (AxisValue :type Float%20%28single-precision%29))
  (Pawn|Input|AddMovementInput "1.000000, 0, 0" AxisValue false))

(fn ConstructionScript)

(fn Flipbook
  ;[1 1 1] Joey's Movement
  (if (or (!= (Input|AxisValues|Getleftandright) 0.0) (!= (Input|AxisValues|Getupanddown) 0.0))
    (Variables|Default|SetJoey_Movements (select (> (Input|AxisValues|Getupanddown) 0.0) "NewEnumerator0" (select (< (Input|AxisValues|Getupanddown) 0.0) "NewEnumerator1" (select (> (Input|AxisValues|Getleftandright) 0.0) "NewEnumerator3" "NewEnumerator2")))))
  (Sprite|SetFlipbook (Variables|Default|GetSprite) (select (> (Math|Vector|VectorLength (Transformation|GetVelocity)) 0.0) (Utilities|Select :Index (Variables|Default|GetJoey_Movements) :NewEnumerator0 "/Game/Spritesheet/MainCharacter_Flipbook/up/up.up" :NewEnumerator1 "/Game/Spritesheet/MainCharacter_Flipbook/down/Down.Down" :NewEnumerator2 "/Game/Spritesheet/MainCharacter_Flipbook/left/left.left" :NewEnumerator3 "/Game/Spritesheet/MainCharacter_Flipbook/right/right.right") (Utilities|Select :Index (Variables|Default|GetJoey_Movements) :NewEnumerator0 "/Game/Spritesheet/MainCharacter_Flipbook/up/idleup.idleup" :NewEnumerator1 "/Game/Spritesheet/MainCharacter_Flipbook/down/idledown.idledown" :NewEnumerator2 "/Game/Spritesheet/MainCharacter_Flipbook/left/idleleft.idleleft" :NewEnumerator3 "/Game/Spritesheet/MainCharacter_Flipbook/right/idleright.idleright"))))